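; Countdown timer actor that shows a decrementing number on a text render, with optional tones.
; StartTimer resets the counter and runs DecrementTimer on a looping function-name timer, updating the text and sound each interval.
; Pausing clears the timer handle, and unpausing creates a fresh timer without resetting the count.
; At zero it shows end text, or zero if blank, plays the end tone, then resets after one interval.
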(event Custom|StartTimer
  ;[1 1 1] Start The Timer - Initialize/Clear the Text Render's text then Clear the Timer Handle, then start the timer and save the timer handle
  (CallFunction|InitializeTimer)
  (CallFunction|ClearTimerHandle)
  (bind _returnvalue (Utilities|Time|SetTimerbyFunctionName 0 "DecrementTimer" (Variables|TimerSettings|GetTimerInterval) true))
  (Variables|Default|SetTimerHandle _returnvalue))

(event Custom|StopTimer
  ;[1 1 1] Stop The Timer - Clear timer, wait the timer interval and then reinitialize the timer. Add code at end if addition functionality is needed when the timer finishes.
  (CallFunction|ClearTimerHandle)
  (Utilities|FlowControl|Delay (Variables|TimerSettings|GetTimerInterval))
  (CallFunction|InitializeTimer))

(event Custom|PauseAndUnPauseTimer
  ;[1 1 1] Pause / UnPause Timer - If Timer is Running, Pause It (By Clearing the Timer Handle). If Timer is Paused, UnPause It.
  (if (Variables|Default|GetTimerPaused?)
    (Variables|Default|SetTimerPaused? false)
    ;[1 1 1] Start The Timer - Initialize/Clear the Text Render's text then Clear the Timer Handle, then start the timer and save the timer handle
    (CallFunction|ClearTimerHandle)
    (bind _returnvalue (Utilities|Time|SetTimerbyFunctionName 0 "DecrementTimer" (Variables|TimerSettings|GetTimerInterval) true))
    (Variables|Default|SetTimerHandle _returnvalue)
    (else
      (Variables|Default|SetTimerPaused? true)
      (CallFunction|ClearTimerHandle))))

(fn ConstructionScript)

(fn InitializeTimer
  ;[1 1 1] Initial Timer - Clear Text Render's Text, Reset Counter and Set Timer Paused Flag to False
  (Rendering|Components|TextRender|SetText (Variables|Default|GetTimer) (Variables|Default|GetTextNull))
  (Variables|Default|SetCounter (Variables|TimerSettings|GetStartingNumber))
  (Variables|Default|SetTimerPaused? false))

(fn DecrementTimer
  ;[1 1 1] Decrement Timer - If Counter > 0, Display Timer Text with Tone and Decrease Counter, If Counter = Zero, End Timer
  (if (!= (Variables|Default|GetCounter) 0)
    (CallFunction|DisplayTimerTextwithTone (Utilities|Text|ToText(Integer) (Variables|Default|GetCounter)) (Variables|Default|GetStartTone))
    (Variables|Default|SetCounter (- (Variables|Default|GetCounter) 1))
    (else
      (CallFunction|EndTImer))))

(fn DisplayTimerTextwithTone
  (params (TextToDisplay :type Text) (ToneToPlay :type Sound%20Base%20Object%20Reference))
  ;[1 1 1] Display Timer Text w/Tone - Display the Timer's Text and Play Tone If Tones Are Enabled
  (Rendering|Components|TextRender|SetText (Variables|Default|GetTimer) TextToDisplay)
  (if (Variables|TimerSettings|GetEnableTones)
    (Audio|PlaySoundatLocation ToneToPlay (Transformation|GetActorLocation self))))

(fn EndTimer
  ;[1 1 1] End Timer - If Text Is Empty, Display Zero, Otherwise Display Ending Text. Next Invoke Stop Timer Event
  (if (Utilities|Enum|Equal(Enum) (Variables|TimerSettings|GetTextToDisplayAtEnd) (Variables|Default|GetTextNull))
    (bind _output_get (Variables|TimerSettings|SetTextToDisplayAtEnd (Variables|Default|GetTextZero))))
  (CallFunction|DisplayTimerTextwithTone _output_get (Variables|Default|GetEndTone))
  (CallFunction|StopTimer))

(fn ClearTimerHandle
  (bind _timerhandle (Variables|Default|GetTimerHandle))
  ;[1 1 1] Clear Timer Handle - If Timer Handle Exists, Clear and Invalidate it. This Stops the Set Timer By Function
  (if (Utilities|Time|IsValidTimerHandle _timerhandle)
    (Utilities|Time|ClearandInvalidateTimerbyHandle _timerhandle)))
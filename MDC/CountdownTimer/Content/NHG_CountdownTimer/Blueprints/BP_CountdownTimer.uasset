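; Countdown timer actor that shows a descending number on a text component, with optional tones at its location.
; It starts on BeginPlay or StartTimer, using a looping timer to call DecrementTimer, which displays the count and plays the start tone each tick.
; At zero it shows configurable end text, defaulting to zero, with an end tone.
; StopTimer then clears the timer and, after one interval, resets text and counter.
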(event Custom|StartTimer
  ;[1 1 1] Start The Timer - Initialize/Clear the Text Render's text then start the timer and save the timer handle
  (CallFunction|InitializeTimer)
  (bind _returnvalue (Utilities|Time|SetTimerbyFunctionName 0 "DecrementTimer" (Variables|TimerSettings|GetTimerInterval) true))
  (Variables|Default|SetTimerHandle _returnvalue))

(event Custom|StopTimer
  ;[1 1 1] Stop The Timer - Clear timer, wait the timer interval and then reinitialize the timer. Add code at end if addition functionality is needed when the timer finishes.
  (Utilities|Time|ClearandInvalidateTimerbyHandle (Variables|Default|GetTimerHandle))
  (Utilities|FlowControl|Delay (Variables|TimerSettings|GetTimerInterval))
  (CallFunction|InitializeTimer))

(event EventBeginPlay
  ;[1 1 1] Start The Timer - Initialize/Clear the Text Render's text then start the timer and save the timer handle
  (CallFunction|InitializeTimer)
  (bind _returnvalue (Utilities|Time|SetTimerbyFunctionName 0 "DecrementTimer" (Variables|TimerSettings|GetTimerInterval) true))
  (Variables|Default|SetTimerHandle _returnvalue))

(fn ConstructionScript)

(fn DecrementTimer
  (if (!= (Variables|Default|GetCounter) 0)
    (CallFunction|DisplayTimerTextwithTone (Utilities|Text|ToText(Integer) (Variables|Default|GetCounter)) (Variables|Default|GetStartTone))
    (Variables|Default|SetCounter (- (Variables|Default|GetCounter) 1))
    (else
      (CallFunction|EndTImer))))

(fn InitializeTimer
  (Rendering|Components|TextRender|SetText (Variables|Default|GetTimer) (Variables|Default|GetTextNull))
  (Variables|Default|SetCounter (Variables|TimerSettings|GetStartingNumber)))

(fn EndTImer
  (if (Utilities|Enum|Equal(Enum) (Variables|TimerSettings|GetTextToDisplayAtEnd) (Variables|Default|GetTextNull))
    (bind _output_get (Variables|TimerSettings|SetTextToDisplayAtEnd (Variables|Default|GetTextZero))))
  (CallFunction|DisplayTimerTextwithTone _output_get (Variables|Default|GetEndTone))
  (CallFunction|StopTimer))

(fn DisplayTimerTextwithTone
  (params (TextToDisplay :type Text) (ToneToPlay :type Sound%20Base%20Object%20Reference))
  (Rendering|Components|TextRender|SetText (Variables|Default|GetTimer) TextToDisplay)
  (if (Variables|TimerSettings|GetEnableTones)
    (Audio|PlaySoundatLocation ToneToPlay (Transformation|GetActorLocation self) "0, 0, 0" 1.0 1.0 0.0 0 0 0)))